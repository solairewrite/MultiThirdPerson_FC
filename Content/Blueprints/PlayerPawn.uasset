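; PlayerPawn is the player-controlled pawn, armed with a grenade launcher and aided by an on-screen crosshair.
; On BeginPlay it spawns BP_GernadeLauncher with itself as owner, stores it as the current weapon, and snaps it to the mesh's WeaponSocket.
; It then creates the WBP_CrossHair widget and adds it to the viewport.
; Pressing the left mouse button calls Fire on the current weapon.
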(event `self.ReceiveBeginPlay`
  (`|ExecutionSequence`
    (:`then_0`
      ;[1 1 1] 设置武器
      (bind _returnvalue (`|SpawnActorFromClass` "/Game/Blueprints/BP_GernadeLauncher.BP_GernadeLauncher_C" (`KismetMathLibrary.MakeTransform` (0.0 0.0 0.0)) "AlwaysSpawn" "OverrideRootScale" self null))
      (set `self.CuttentWeapon` _returnvalue)
      (`self.K2_AttachToComponent` _returnvalue (`self.Mesh`) "WeaponSocket" "SnapToTarget" "SnapToTarget" "SnapToTarget" true))
    (:`then_1`
      ;[1 1 1] 准星UI
      (bind _returnvalue_2 (`|CreateWidget` "/Game/UI/WBP_CrossHair.WBP_CrossHair_C"))
      (`UserWidget.AddToViewport` _returnvalue_2 0))))

(event `Key|LeftMouseButton`
  (params (Key :type "Key Structure"))
  ;[1 1 1] 左键开火
  (:`Pressed`
    (`SWeapon.Fire` (`self.CuttentWeapon`))))

(fn `UserConstructionScript`)