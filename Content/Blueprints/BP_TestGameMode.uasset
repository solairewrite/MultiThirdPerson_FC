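; Test game mode that spawns AI bots and awards score for killing them.
; SpawnNewBot runs an EQS query for a location, then spawns either an advanced AI or a tracker bot there by weighted random choice, with a debug sphere marking the spot.
; An actor-killed event, bound on BeginPlay, adds score to the killer's SPlayerState when the victim is a non-player pawn, then prints the total.
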(event `self.SpawnNewBot`
  ;[1 1 1] EQS查找生成点,创建Bot
  (bind _returnvalue (`EnvQueryManager.RunEQSQuery` "/Game/AI/EQS_FindSpawnLocation.EQS_FindSpawnLocation" self "SingleResult"))
  (add `EnvQueryInstanceBlueprintWrapper.OnQueryFinishedEvent` _returnvalue (delegate `OnQueryFinished`)))

(event `OnQueryFinished`
  (params (QueryInstance :type "EnvQueryInstanceBlueprintWrapper Object Reference") (QueryStatus :type "EEnvQueryStatus Enum" :default "Processing"))
  ;[1 1 1] EQS查找生成点,创建Bot
  (switch `EEnvQueryStatus` QueryStatus
    (:`Success`
      (for _array_element (`EnvQueryInstanceBlueprintWrapper.GetResultsAsLocations` QueryInstance)
        (`KismetSystemLibrary.DrawDebugSphere` _array_element 50.0 12 (struct :`R` 1.0 :`G` 0.772992 :`A` 1.0) 2.0 2.0)
        (bind _returnvalue (`|SpawnActorFromClass` (select `bool` (<= (`KismetMathLibrary.RandomFloatInRange` 0.0 100.0) 35.0) :`false` "/Game/AI/TrackerBot/BP_TrackerBot.BP_TrackerBot_C" :`true` "/Game/AI/AdvancedAI/BP_AdvancedAI.BP_AdvancedAI_C" :!type "Actor Class Reference") (`KismetMathLibrary.MakeTransform` _array_element) "AdjustIfPossibleButDontSpawnIfColliding" "OverrideRootScale" null null))))))

(event `self.ReceiveBeginPlay`
  (add `self.onActorKilled` (delegate `OnActorKillEvent`)))

(event `OnActorKillEvent` :!signature `self.onActorKilled`
  (params (VictimActor :type "Actor Object Reference") (KillerActor :type "Actor Object Reference") (KillerController :type "Controller Object Reference"))
  (bind _aspawn (cast `Pawn` VictimActor))
  (if (not (`Pawn.IsPlayerControlled` _aspawn))
    (`/Engine/EditorBlueprintResources/StandardMacros.IsValid` KillerController
      (:`Is Valid`
        (bind _assplayer_state (cast `SPlayerState` (`Pawn.PlayerState` (`Controller.K2_GetPawn` KillerController))))
        (`SPlayerState.AddScore` _assplayer_state 20.0)
        (`KismetSystemLibrary.PrintString` (`KismetStringLibrary.Conv_DoubleToString` (`PlayerState.Score` _assplayer_state)) true true (struct :`R` 0.204749 :`G` 0.483333 :`B` 0.119013 :`A` 1.0))))))

(fn `UserConstructionScript`)